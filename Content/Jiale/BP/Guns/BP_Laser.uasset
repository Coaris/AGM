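; BP_Laser is a laser actor that draws a red Niagara beam along its forward vector.
; On BeginPlay it sets the beam's color and width parameters.
; Each Tick it line traces on the Camera channel out to Distance and sets the beam end to the blocking hit location, or to the trace end otherwise.
; The trace also draws a one-frame debug line.
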(event `self.ReceiveBeginPlay`
  (bind _niagara_laser (`self.Niagara_Laser`))
  (`FXSystemComponent.SetColorParameter` _niagara_laser "Color" (struct :`R` 0.992 :`A` 1.0))
  (`FXSystemComponent.SetFloatParameter` _niagara_laser "laserWidth" 1.0))

(event `self.ReceiveTick`
  (params (DeltaSeconds :type "Float (single-precision)"))
  (bind _returnvalue (`self.K2_GetActorLocation`))
  (bind _returnvalue_2 (+ _returnvalue (* (`self.GetActorForwardVector`) (`self.distance`))))
  (set `self.traceEnd` _returnvalue_2)
  (bind _outhit (`KismetSystemLibrary.LineTraceSingle` :`Start` _returnvalue :`End` _returnvalue_2 :`TraceChannel` "TraceTypeQuery2" :`DrawDebugType` "ForOneFrame"))
  (`FXSystemComponent.SetVectorParameter` (`self.Niagara_Laser`) "laserEnd" (select `bool` (`GameplayStatics.BreakHitResult` _outhit) :`false` (`self.traceEnd`) :`true` (`.Location` (`GameplayStatics.BreakHitResult` _outhit)))))

(fn `UserConstructionScript`)