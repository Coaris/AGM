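; BP_Revolver_L is the left-hand revolver, binding the player controller's left shoot and reload events on BeginPlay.
; It relies on inherited gun logic for shooting and reloading.
; A successful shot plays a timeline that kicks the actor along relative X and updates the left bullet count on the HUD each update.
; Reload runs a second timeline that drives PlayReloadAnim.
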(event `self.ReceiveBeginPlay`
  (`parent.ReceiveBeginPlay`)
  ;[1 1 1] 左手开枪事件
  (add `/Game/Jiale/BP/BP_PlayerController.OnShoot_L` (`self.playerController_BP`) (delegate `OnShoot_L_Event`))
  ;[1 1 1] 左手换弹事件
  (add `/Game/Jiale/BP/BP_PlayerController.OnReload_L` (`self.playerController_BP`) (delegate `OnReload_L_Event`)))

(event `OnReload_L_Event`
  ;[1 1 1] 左手换弹事件
  (`self.Reload`)
  ;;[1 1 1] 换弹动画
  (bind (_direction _reloadanim) (`Timeline|Timeline_0` :!via `PlayFromStart`)
    (:`Update`
      (`self.Play Reload Anim` _reloadanim))))

(event `OnShoot_L_Event`
  ;[1 1 1] 左手开枪事件
  (bind _shot (`self.Shoot`))
  ;;[1 1 1] 开枪动画
  (if _shot
    (bind (_direction _shootanim) (`Timeline|ShootAnimation` :!via `PlayFromStart`)
      (:`Update`
        (`self.K2_SetActorRelativeLocation` (`KismetMathLibrary.MakeVector` (* _shootanim -10.0)))
        ;;[1 1 1] ShootAnim_UI
        ;;;[1 0.03585 0] ???
        (message `/Game/Jiale/UI/Gaming/BPI_HUD.ChangeUI_Left_Shoot` (`self.HUD_WBP`) (`self.bulletCount`))))))

(event `self.ReceiveTick`
  (params (DeltaSeconds :type "Float (single-precision)"))
  (`parent.ReceiveTick` DeltaSeconds))

(fn `UserConstructionScript`
  (`parent.UserConstructionScript`))