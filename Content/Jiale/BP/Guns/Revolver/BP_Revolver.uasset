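; BP_Revolver is a revolver gun actor that tracks a four-round magazine and handles firing and reloading feedback.
; Shoot uses CheckMagazine to clamp the count and detect empty, then either plays a dry-fire sound or spends a round with sound and camera shake, returning whether it fired.
; Reload refills instantly with a sound, while PlayReloadAnim pitches the barrel from a passed-in timeline value.
; BeginPlay caches the BP_PlayerController.
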(event `self.ReceiveBeginPlay`
  (bind _outactors (`GameplayStatics.GetAllActorsOfClass` "/Game/Jiale/BP/BP_PlayerController.BP_PlayerController_C"))
  (set `self.playerController_BP` (`|GetArrayItem` _outactors)))

(fn `CheckMagazine`
  (params (bulletCount :type Integer))
  (returns (isMagazineEmpty :type Boolean))
  ;[1 1 1] 对应手子弹为空时，返回True，否则返回False
  (`|ExecutionSequence`
    (:`then_0`
      ;[1 1 1] 防溢出
      (if (>= bulletCount 4)
        (set `self.bulletCount` 4)))
    (:`then_1`
      (if (<= bulletCount 0)
        (set `self.bulletCount` 0)
        (return true)
        (else
          (return false))))))

(fn `Play Reload Anim`
  (params (ReloadTimeline :type "Float (double-precision)"))
  (`SceneComponent.K2_SetRelativeRotation` (`self.Barrel`) (`KismetMathLibrary.MakeRotator` 0.0 (* ReloadTimeline -90.0)) false false))

(fn `Reload`
  (`GameplayStatics.PlaySound2D` "/Game/Jiale/SFX/Revolver/Revolver_Reload.Revolver_Reload" 1.0 1.0 0.0 null null)
  (set `self.bulletCount` 4))

(fn `Shoot`
  (returns (Shot :type Boolean))
  (bind _bulletcount (`self.bulletCount`))
  ;[1 1 1] 开枪逻辑——据剩余子弹，是否开枪
  (bind _ismagazineempty (`self.CheckMagazine` _bulletcount))
  (if _ismagazineempty
    (`GameplayStatics.PlaySound2D` "/Game/Jiale/SFX/Revolver/Revolver_Empty.Revolver_Empty" 1.0 1.0 0.0 null null)
    (return false) ; 无法开枪
    (else
      (set `self.bulletCount` (- _bulletcount 1))
      ;[1 1 1] 开枪音效
      (`GameplayStatics.PlaySound2D` "/Game/Jiale/SFX/Revolver/Revolver_Shoot.Revolver_Shoot" 1.0 1.0 0.0 null null)
      ;[1 1 1] 开枪屏幕抖动
      (`LegacyCameraShake.StartLegacyCameraShake` (`GameplayStatics.GetPlayerCameraManager` 0) "/Game/Jiale/BP/BP_CameraShake_Shoot.BP_CameraShake_Shoot_C")
      (return true) ; 成功开枪
    )))

(fn `UserConstructionScript`)