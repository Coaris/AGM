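; Right-hand revolver gun Blueprint that handles firing and reloading with animation and HUD feedback.
; On BeginPlay it binds to the player controller's right shoot and reload delegates.
; A successful shot plays a recoil timeline on relative X, updates the HUD and decrements the bullet count, while a failed shot shows an empty-gun HUD message.
; Reload drives an animation timeline and notifies the HUD at start and finish.
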(event `self.ReceiveBeginPlay`
  (`parent.ReceiveBeginPlay`)
  ;[1 1 1] 右手开枪事件
  (add `/Game/Jiale/BP/BP_PlayerController.OnShoot_R` (`self.playerController_BP`) (delegate `OnShoot_R_Event`))
  ;[1 1 1] 右手换弹事件
  (add `/Game/Jiale/BP/BP_PlayerController.OnReload_R` (`self.playerController_BP`) (delegate `OnReload_R_Event`)))

(event `OnShoot_R_Event`
  (bind _bulletcount (`self.bulletCount`))
  ;[1 1 1] 右手开枪事件
  (bind _shot (`self.Shoot`))
  (if _shot
    (`|ExecutionSequence`
      (:`then_0`
        ;;[1 1 1] 开枪动画
        (bind (_direction _shootanim) (`Timeline|ShootAnimation` :!via `PlayFromStart`)
          (:`Update`
            (`self.K2_SetActorRelativeLocation` (`KismetMathLibrary.MakeVector` (* _shootanim -10.0))))))
      (:`then_1`
        ;;[1 1 1] ShootAnim_UI
        (message `/Game/Jiale/UI/Gaming/BPI_HUD.ChangeHUD_Right_Shoot` (`self.HUD_WBP`) _bulletcount)
        (set `self.bulletCount` (- _bulletcount 1))))
    (else
      ;;[1 1 1] 播放HUD右手空枪动画
      (message `/Game/Jiale/UI/Gaming/BPI_HUD.ChangeHUD_Right_Empty` (`self.HUD_WBP`)))))

(event `OnReload_R_Event`
  ;[1 1 1] 右手换弹事件
  (`self.Reload`)
  (`|ExecutionSequence`
    (:`then_0`
      ;;[1 1 1] 换弹动画
      (bind (_direction _reloadanim) (`Timeline|ReloadAnimation` :!via `PlayFromStart`)
        (:`Update`
          (`self.Play Reload Anim` _reloadanim))
        (:`Finished`
          (message `/Game/Jiale/UI/Gaming/BPI_HUD.ChangeHUD_Right_Reload_End` (`self.HUD_WBP`)))))
    (:`then_1`
      (message `/Game/Jiale/UI/Gaming/BPI_HUD.ChangeHUD_Right_Reload` (`self.HUD_WBP`)))))

(fn `UserConstructionScript`
  (`parent.UserConstructionScript`))