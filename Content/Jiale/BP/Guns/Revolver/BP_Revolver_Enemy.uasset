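; Enemy revolver Blueprint that provides shooting and reloading, though its event graph is a stub: ShootPlayer only prints a debug string and the delayed firing loop is disconnected.
; Shoot checks the magazine, then plays sound and camera shake and spawns a muzzle bullet, without decrementing BulletCount.
; Reload spawns bullet actors from four ejectors and refills the count.
; PlayReloadAnim pitches the barrel from a supplied timeline value.
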(event `self.ReceiveTick`
  (params (DeltaSeconds :type "Float (single-precision)")))

(event `/Game/Jiale/BP/Guns/Revolver/BPI_Revolver.ShootPlayer`
  (`KismetSystemLibrary.PrintString` "Hello"))

(fn `CheckMagazine`
  (params (bulletCount :type Integer))
  (returns (isMagazineEmpty :type Boolean))
  ;[1 1 1] 对应手子弹为空时，返回True，否则返回False
  (`|ExecutionSequence`
    (:`then_0`
      ;[1 1 1] 防溢出
      (if (>= bulletCount 4)
        (set `self.bulletCount` 4)))
    (:`then_1`
      (if (<= bulletCount 0)
        (set `self.bulletCount` 0)
        (return true)
        (else
          (return false))))))

(fn `Play Reload Anim`
  (params (ReloadTimeline :type "Float (double-precision)"))
  (`SceneComponent.K2_SetRelativeRotation` (`self.Barrel`) (`KismetMathLibrary.MakeRotator` 0.0 (* ReloadTimeline -90.0)) false false))

(fn `Reload`
  (bind (_returnvalue_location _returnvalue_rotation) (`KismetMathLibrary.BreakTransform` (`SceneComponent.K2_GetComponentToWorld` (`self.Bullet_Ejector_L`))))
  (bind (_returnvalue_location_2 _returnvalue_rotation_2) (`KismetMathLibrary.BreakTransform` (`SceneComponent.K2_GetComponentToWorld` (`self.Bullet_Ejector_U`))))
  (bind (_returnvalue_location_3 _returnvalue_rotation_3) (`KismetMathLibrary.BreakTransform` (`SceneComponent.K2_GetComponentToWorld` (`self.Bullet_Ejector_R`))))
  (bind (_returnvalue_location_4 _returnvalue_rotation_4) (`KismetMathLibrary.BreakTransform` (`SceneComponent.K2_GetComponentToWorld` (`self.Bullet_Ejector_D`))))
  (`GameplayStatics.PlaySound2D` "/Game/Jiale/SFX/Revolver/Revolver_Reload.Revolver_Reload" 1.0 1.0 0.0 null null)
  (`|ExecutionSequence`
    (:`then_0`
      (`|SpawnActorFromClass` "/Game/Jiale/BP/Guns/Bullet/BP_Bullet_Reload.BP_Bullet_Reload_C" (`KismetMathLibrary.MakeTransform` _returnvalue_location_3 _returnvalue_rotation_3) "AlwaysSpawn" "MultiplyWithRoot" null null))
    (:`then_1`
      (`|SpawnActorFromClass` "/Game/Jiale/BP/Guns/Bullet/BP_Bullet_Reload.BP_Bullet_Reload_C" (`KismetMathLibrary.MakeTransform` _returnvalue_location_4 _returnvalue_rotation_4) "AlwaysSpawn" "MultiplyWithRoot" null null))
    (:`then_2`
      (`|SpawnActorFromClass` "/Game/Jiale/BP/Guns/Bullet/BP_Bullet_Reload.BP_Bullet_Reload_C" (`KismetMathLibrary.MakeTransform` _returnvalue_location _returnvalue_rotation) "AlwaysSpawn" "MultiplyWithRoot" null null))
    (:`then_3`
      (`|SpawnActorFromClass` "/Game/Jiale/BP/Guns/Bullet/BP_Bullet_Reload.BP_Bullet_Reload_C" (`KismetMathLibrary.MakeTransform` _returnvalue_location_2 _returnvalue_rotation_2) "AlwaysSpawn" "MultiplyWithRoot" null null)
      (set `self.bulletCount` 4))))

(fn `Shoot`
  (returns (Shot :type Boolean))
  (bind (_returnvalue_location _returnvalue_rotation) (`KismetMathLibrary.BreakTransform` (`SceneComponent.K2_GetComponentToWorld` (`self.Muzzle`))))
  ;[1 1 1] 开枪逻辑——据剩余子弹，是否开枪
  (bind _ismagazineempty (`self.CheckMagazine` (`self.bulletCount`)))
  (if _ismagazineempty
    (return false) ; 无法开枪
    (else
      ;[1 1 1] 开枪音效
      (`GameplayStatics.PlaySound2D` "/Game/Jiale/SFX/Revolver/Revolver_Shoot.Revolver_Shoot" 1.0 1.0 0.0 null null)
      ;[1 1 1] 开枪屏幕抖动
      (`LegacyCameraShake.StartLegacyCameraShake` (`GameplayStatics.GetPlayerCameraManager` 0) "/Game/Jiale/BP/BP_CameraShake_Shoot.BP_CameraShake_Shoot_C")
      ;[1 1 1] 射出子弹实体
      (`|SpawnActorFromClass` "/Game/Jiale/BP/Guns/Bullet/BP_Bullet_Shoot.BP_Bullet_Shoot_C" (`KismetMathLibrary.MakeTransform` _returnvalue_location _returnvalue_rotation) "AlwaysSpawn" "MultiplyWithRoot" null null)
      (return true) ; 成功开枪
    )))

(fn `UserConstructionScript`)