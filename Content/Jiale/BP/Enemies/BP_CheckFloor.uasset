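; BP_CheckFloor is a one-shot trigger zone that wakes an assigned list of enemies in response to BP_Bill.
; While Bill overlaps the CheckFloor component, either of the player controller's left or right shoot events triggers it.
; Unless flagged IsOutside, staying inside until the InTimer timeline finishes also triggers it, and leaving stops that timer.
; TriggerByKill offers another entry point, setting IsTriggered and each valid enemy's IsWaked.
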(event `self.ReceiveBeginPlay`
  (bind _playercontroller (`self.playerController`))
  ;[1 1 1] 获得BP_PlayerController
  (bind _asbp_player_controller (cast `/Game/Jiale/BP/BP_PlayerController` (`GameplayStatics.GetPlayerController` 0)))
  (set `self.playerController` _asbp_player_controller)
  (add `/Game/Jiale/BP/BP_PlayerController.OnShoot_L` _playercontroller (delegate `OnShoot_L_Event`))
  (add `/Game/Jiale/BP/BP_PlayerController.OnShoot_R` _playercontroller (delegate `OnShoot_R_Event`)))

(event `OnShoot_L_Event`
  (if (`self.isTriggered`) :!label _label
    _
    (elif (`self.isIn`)
      (set `self.isTriggered` true :!label _label_2)
      (for _array_element (`self.enemyList`)
        (`/Engine/EditorBlueprintResources/StandardMacros.IsValid` _array_element
          (:`Is Valid`
            (set `/Game/Jiale/BP/Enemies/BP_Enemy_Normal.isWaked` true _array_element)))))))

(event `OnShoot_R_Event`
  (goto _label))

(event `TriggerByKill`
  (goto _label_2))

(event `TriggerByTime`
  (goto _label_2))

(event `self.CheckFloor.OnComponentBeginOverlap`
  (params (OverlappedComponent :type "PrimitiveComponent Object Reference") (OtherActor :type "Actor Object Reference") (OtherComp :type "PrimitiveComponent Object Reference") (OtherBodyIndex :type Integer) (bFromSweep :type Boolean) (SweepResult :type "HitResult Structure (by ref)"))
  (if (not (`self.isTriggered`))
    (cast `/Game/Jiale/BP/Bill/BP_Bill` OtherActor)
    (set `self.isIn` true)
    (if (not (`self.isOutside`))
      (`Timeline|InTimer` :!via `PlayFromStart` :!label _label_3
        (:`Finished`
          (`self.TriggerByTime`))))))

(event `self.CheckFloor.OnComponentEndOverlap`
  (params (OverlappedComponent :type "PrimitiveComponent Object Reference") (OtherActor :type "Actor Object Reference") (OtherComp :type "PrimitiveComponent Object Reference") (OtherBodyIndex :type Integer))
  (if (not (`self.isTriggered`))
    (cast `/Game/Jiale/BP/Bill/BP_Bill` OtherActor)
    (set `self.isIn` false)
    (if (not (`self.isOutside`))
      (goto _label_3 :!via `Stop`))))

(fn `UserConstructionScript`)