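; BP_Enemy_Normal is an enemy that carries a revolver and, once woken, turns to face the player.
; BeginPlay caches the player and attaches a spawned BP_Revolver_Enemy to a body socket.
; While awake, Tick line-traces at a fixed height and compares the first hit to the player by display name, but nothing follows a match yet.
; On EndPlay it calls TriggerByKill on CheckFloor to wake others in the room.
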(event `self.ReceiveBeginPlay`
  (`|ExecutionSequence`
    (:`then_0`
      ;[1 1 1] 获得玩家引用
      (bind _ascharacter (cast `Character` (`GameplayStatics.GetPlayerPawn` 0)))
      (set `self.player` _ascharacter)
      ;[1 1 1] 被杀时，唤醒房间其他人
      (add `self.OnEndPlay` (delegate `OnEndPlay_Event`)))
    (:`then_1`
      ;[1 1 1] Spawn a Revolver
      (bind _returnvalue (`|SpawnActorFromClass` "/Game/Jiale/BP/Guns/Revolver/BP_Revolver_Enemy.BP_Revolver_Enemy_C" (`SceneComponent.GetSocketTransform` (`self.Body`) "RevolverPosition" "RTS_Actor") "AlwaysSpawn" "MultiplyWithRoot" null null))
      (bind _output_get (set `self.revolver` _returnvalue))
      (`self.K2_AttachToComponent` _output_get (`self.Body`) "RevolverPosition" "SnapToTarget" "SnapToTarget" "SnapToTarget" true))))

(event `OnEndPlay_Event` :!signature `self.OnEndPlay`
  (params (Actor :type "Actor Object Reference") (EndPlayReason :type "EEndPlayReason Enum" :default "Destroyed"))
  (bind _checkfloor (`self.checkFloor`))
  ;[1 1 1] 被杀时，唤醒房间其他人
  (`/Engine/EditorBlueprintResources/StandardMacros.IsValid` _checkfloor
    (:`Is Valid`
      (`/Game/Jiale/BP/Enemies/BP_CheckFloor.TriggerByKill` _checkfloor))))

(event `self.ReceiveTick`
  (params (DeltaSeconds :type "Float (single-precision)"))
  (bind (_returnvalue_x _returnvalue_y) (`KismetMathLibrary.BreakVector` (`self.K2_GetActorLocation`)))
  (bind _returnvalue (`self.K2_GetActorLocation` (`self.player`)))
  (bind (_x _y) (`KismetMathLibrary.BreakVector3f` _returnvalue))
  ;[1 1 1] 是否被唤醒
  (if (`self.isWaked`)
    ;[1 1 1] 看向玩家
    (`self.K2_SetActorRotation` (`KismetMathLibrary.FindLookAtRotation` (`self.K2_GetActorLocation`) _returnvalue))
    ;[1 1 1] 射线检测是否看到玩家
    (bind _outhits (`KismetSystemLibrary.LineTraceMulti` :`Start` (`KismetMathLibrary.MakeVector` _returnvalue_x _returnvalue_y 80.0) :`End` (`KismetMathLibrary.MakeVector` _x _y 80.0) :`TraceChannel` "TraceTypeQuery4" :`DrawDebugType` "ForOneFrame"))
    (bind (_output_bblockinghit _output_binitialoverlap _output_time _output_distance _output_location _output_impactpoint _output_normal _output_impactnormal _output_physmat _output_hitactor) (`GameplayStatics.BreakHitResult` (`|GetArrayItem` _outhits)))
    ;[1 1 1] If the first actor is player
    (if (`KismetStringLibrary.EqualEqual_StrStr` (`KismetSystemLibrary.GetDisplayName` _output_hitactor) (`KismetSystemLibrary.GetDisplayName` (`self.player`)))
      _)))

(fn `UserConstructionScript`)