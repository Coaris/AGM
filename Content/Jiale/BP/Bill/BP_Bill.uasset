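; BP_Bill is a player character that moves, dashes and aims both arms at a target point.
; Enhanced Input movement follows horizontal axes taken from the level's "StartCamera".
; Dash adds an unswept offset each Tick from the last move direction, with timelines timing duration and cooldown.
; The Lookat event turns Bill toward the target and blends the shoulders from spread sideways to straight ahead as distance grows from FocusMin to FocusMax.
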(event `self.ReceiveBeginPlay`
  (bind _startcamera (`self.startCamera`))
  (bind (_returnvalue_x _returnvalue_y) (`KismetMathLibrary.BreakVector` (`self.GetActorForwardVector` _startcamera)))
  ;[1 1 1] 获得关卡相机的引用
  (bind _outactors (`GameplayStatics.GetAllActorsOfClass` "/Script/Engine.CameraActor"))
  (for _array_element _outactors
    (if (`KismetStringLibrary.EqualEqual_StrStr` (`KismetSystemLibrary.GetDisplayName` _array_element) "StartCamera")
      (set `self.startCamera` _array_element)
      ;[1 1 1] 获得MainCamera前向量的水平分量&右分量
      (set `self.levelRightVector` (`self.GetActorRightVector` _startcamera))
      (set `self.levelForwardVector` (`KismetMathLibrary.Normal` (`KismetMathLibrary.MakeVector` _returnvalue_x _returnvalue_y))))))

(event `self.ReceiveTick`
  (params (DeltaSeconds :type "Float (single-precision)"))
  (bind _move_direction (`self.move Direction`))
  ;[1 1 1] 冲刺，位移逻辑
  (if (`self.isDashing`)
    (`self.K2_AddActorWorldOffset` (* (`KismetMathLibrary.MakeVector` (`KismetMathLibrary.Dot_VectorVector` (`self.levelForwardVector`) _move_direction) (`KismetMathLibrary.Dot_VectorVector` _move_direction (`self.levelRightVector`))) (`self.dashDistance`)))))

(event `EnhancedInput|/Game/Jiale/Input/IA_Move`
  (params (ActionValue :type "Vector2D Structure") (ElapsedSeconds :type "Float (double-precision)") (TriggeredSeconds :type "Float (double-precision)") (InputAction :type "InputAction Object Reference" :default "/Game/Jiale/Input/IA_Move.IA_Move"))
  (bind (_returnvalue_x _returnvalue_y) (`KismetMathLibrary.BreakVector2D` (`KismetMathLibrary.Normal2D` ActionValue)))
  ;[1 1 1] 使用EIS移动
  (:`Triggered`
    (bind _output_get (set `self.move Direction` (`KismetMathLibrary.MakeVector` _returnvalue_y _returnvalue_x)))
    (`|ExecutionSequence`
      (:`then_0`
        (`self.AddMovementInput` (`self.levelRightVector`) (.y _output_get)))
      (:`then_1`
        (`self.AddMovementInput` (`self.levelForwardVector`) (.x _output_get))))))

(event `EnhancedInput|/Game/Jiale/Input/IA_Dash`
  (params (ActionValue :type Boolean) (ElapsedSeconds :type "Float (double-precision)") (TriggeredSeconds :type "Float (double-precision)") (InputAction :type "InputAction Object Reference" :default "/Game/Jiale/Input/IA_Dash.IA_Dash"))
  ;[1 1 1] 冲刺
  (:`Triggered`
    (if (`self.isDashReady`)
      (set `self.isDashReady` false)
      (set `self.isDashing` true)
      (`|ExecutionSequence`
        (:`then_0`
          ;;[1 1 1] 冲刺时间
          (`Timeline|DashDuration` :!via `PlayFromStart`
            (:`Finished`
              (set `self.isDashing` false))))
        (:`then_1`
          ;;[1 1 1] 冲刺CD
          (`Timeline|DashCD` :!via `PlayFromStart`
            (:`Finished`
              (set `self.isDashReady` true))))))))

(event `/Game/Jiale/BP/Bill/BPI_Bill.LookAt`
  (params (AimTarget :type "Vector Structure"))
  (bind (_returnvalue_x _returnvalue_y) (`KismetMathLibrary.BreakVector` (`self.K2_GetActorLocation`)))
  (bind (_returnvalue_x_2 _returnvalue_y_2) (`KismetMathLibrary.BreakVector` (`self.K2_GetActorLocation`)))
  (bind _focusmin (`self.focusMin`))
  (bind _returnvalue (`KismetMathLibrary.Vector_Distance` (`KismetMathLibrary.MakeVector` AimTarget_X AimTarget_Y) (`KismetMathLibrary.MakeVector` _returnvalue_x_2 _returnvalue_y_2)))
  ;[1 1 1] 玩家看到鼠标位置
  (`self.K2_SetActorRotation` (`KismetMathLibrary.FindLookAtRotation` (`KismetMathLibrary.MakeVector` _returnvalue_x _returnvalue_y) (`KismetMathLibrary.MakeVector` AimTarget_X AimTarget_Y)))
  ;[1 1 1] 调整瞄准角度
  ;;[1 1 1] 当鼠标距离比小焦距小时
  (if (<= _returnvalue (`self.focusMin`))
    ;;[1 1 1] 两侧展开双臂
    (`|ExecutionSequence`
      (:`then_0`
        (`SceneComponent.K2_SetRelativeRotation` (`self.Shoulder_L`) (`KismetMathLibrary.MakeRotator` 0.0 0.0 -90.0) false false))
      (:`then_1`
        (`SceneComponent.K2_SetRelativeRotation` (`self.Shoulder_R`) (`KismetMathLibrary.MakeRotator` 0.0 0.0 90.0) false false)))
    (else
      ;;[1 1 1] 当鼠标距离比大焦距大时
      (if (>= _returnvalue (`self.focusMax`))
        ;;[1 1 1] 向前伸直双臂
        (`|ExecutionSequence`
          (:`then_0`
            (`SceneComponent.K2_SetRelativeRotation` (`self.Shoulder_L`) (`KismetMathLibrary.MakeRotator` 0.0) false false))
          (:`then_1`
            (`SceneComponent.K2_SetRelativeRotation` (`self.Shoulder_R`) (`KismetMathLibrary.MakeRotator` 0.0) false false)))
        (elif true
          ;;[1 1 1] 夹角双臂
          (set `self.aimAlpha` (/ (- _returnvalue _focusmin) (- (`self.focusMax`) _focusmin)))
          (`|ExecutionSequence`
            (:`then_0`
              (`SceneComponent.K2_SetRelativeRotation` (`self.Shoulder_L`) (`KismetMathLibrary.MakeRotator` 0.0 0.0 (- (* (`self.aimAlpha`) 90.0) 90.0)) false false))
            (:`then_1`
              (`SceneComponent.K2_SetRelativeRotation` (`self.Shoulder_R`) (`KismetMathLibrary.MakeRotator` 0.0 0.0 (- 90.0 (* (`self.aimAlpha`) 90.0))) false false))))))))

(fn `UserConstructionScript`)