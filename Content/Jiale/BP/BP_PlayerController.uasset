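; Player controller for dual-handed shooting of BP_Bill, with time slowed except while shooting.
; Tick sends the cursor hit location to Bill's LookAt.
; Enhanced Input shots fire per-hand dispatchers and restore normal time until that hand's cooldown timeline finishes.
; The reload input arms reload mode, where a shoot input reloads that hand and a second reload press reloads both, with timelines gating each hand.
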(event `self.ReceiveBeginPlay`
  (`|ExecutionSequence`
    (:`then_0`
      (`GameplayStatics.SetGlobalTimeDilation` 0.1))
    (:`then_1`
      ;[1 1 1] 获取场景中名为Killer Bill实例的BP_Bill
      (bind _outactors (`GameplayStatics.GetAllActorsOfClass` "/Game/Jiale/BP/Bill/BP_Bill.BP_Bill_C"))
      (set `self.bill_BP_Instance` (`|GetArrayItem` _outactors)))
    (:`then_2`
      ;[1 1 1] 获取IMC
      (`EnhancedInputSubsystemInterface.AddMappingContext` (pcsubsystem `EnhancedInputLocalPlayerSubsystem` (`GameplayStatics.GetPlayerController` 0)) "/Game/Jiale/Input/IMC_Player.IMC_Player" 0 (struct)))
    (:`then_3`
      (set `self.bShowMouseCursor` true))))

(event `self.ReceiveTick`
  (params (DeltaSeconds :type "Float (single-precision)"))
  ;[1 1 1] 将鼠标位置传递给BPI_Bill的LookAt
  (message `/Game/Jiale/BP/Bill/BPI_Bill.LookAt` (`self.bill_BP_Instance`) (`.Location` (`GameplayStatics.BreakHitResult` (`self.GetHitResultUnderCursorByChannel` "TraceTypeQuery1")))))

(event `EnhancedInput|/Game/Jiale/Input/IA_Shoot_L`
  (params (ActionValue :type Boolean) (ElapsedSeconds :type "Float (double-precision)") (TriggeredSeconds :type "Float (double-precision)") (InputAction :type "InputAction Object Reference" :default "/Game/Jiale/Input/IA_Shoot_L.IA_Shoot_L"))
  ;[1 1 1] 左右手分别射击&左右手分别换弹匣事件触发
  (:`Triggered`
    (if (`self.isReloadReady`)
      ;;[1 1 1] 换弹
      (`self.Event Reload L`)
      (set `self.isReloadReady` false :!label _label)
      (else
        ;;[1 1 1] 射击
        (if (`self.isShootReady_L`)
          (if (not (`self.isUsing_L`))
            (set `self.isUsing_L` true)
            (set `self.isShootReady_L` false)
            (`self.OnShoot_L`)
            (`GameplayStatics.SetGlobalTimeDilation` 1.0)
            (`Timeline|ShootCD_L` :!via `PlayFromStart`
              (:`Finished`
                (set `self.isShootReady_L` true)
                (set `self.isUsing_L` false)
                (`GameplayStatics.SetGlobalTimeDilation` 0.1)))))))))

(event `EnhancedInput|/Game/Jiale/Input/IA_Shoot_R`
  (params (ActionValue :type Boolean) (ElapsedSeconds :type "Float (double-precision)") (TriggeredSeconds :type "Float (double-precision)") (InputAction :type "InputAction Object Reference" :default "/Game/Jiale/Input/IA_Shoot_R.IA_Shoot_R"))
  ;[1 1 1] 左右手分别射击&左右手分别换弹匣事件触发
  (:`Triggered`
    (if (`self.isReloadReady`)
      ;;[1 1 1] 换弹
      (`self.Event Reload R`)
      (goto _label)
      (else
        ;;[1 1 1] 射击
        (if (`self.isShootReady_R`)
          (if (not (`self.isUsing_R`))
            (set `self.isUsing_R` true)
            (set `self.isShootReady_R` false)
            (`self.OnShoot_R`)
            (`GameplayStatics.SetGlobalTimeDilation` 1.0)
            (`Timeline|Timeline` :!via `PlayFromStart`
              (:`Finished`
                (set `self.isShootReady_R` true)
                (set `self.isUsing_R` false)
                (`GameplayStatics.SetGlobalTimeDilation` 0.1)))))))))

(event `Event Reload L`
  ;[1 1 1] 换弹
  (if (not (`self.isUsing_L`)) :!label _label_2
    (set `self.isUsing_L` true)
    (`self.OnReload_L`)
    (`Timeline|Reloading_L` :!via `PlayFromStart`
      (:`Finished`
        (set `self.isUsing_L` false)))))

(event `Event Reload Both`
  ;[1 1 1] 换弹
  (`|ExecutionSequence`
    (:`then_0`
      (goto _label_2))
    (:`then_1`
      (if (not (`self.isUsing_R`)) :!label _label_3
        (set `self.isUsing_R` true)
        (`self.OnReload_R`)
        (`Timeline|Reloading_R` :!via `PlayFromStart`
          (:`Finished`
            (set `self.isUsing_R` false)))))))

(event `Event Reload R`
  ;[1 1 1] 换弹
  (goto _label_3))

(event `/Game/Jiale/BP/Guns/Revolver/BPI_Revolver.SendMagFull_L`
  (params (isMagFull_L :type Boolean))
  ;[1 1 1] 换弹
)

(event `/Game/Jiale/BP/Guns/Revolver/BPI_Revolver.SendMagFull_R`
  (params (isMagFull_R :type Boolean))
  ;[1 1 1] 换弹
)

(event `EnhancedInput|/Game/Jiale/Input/IA_Reload`
  (params (ActionValue :type Boolean) (ElapsedSeconds :type "Float (double-precision)") (TriggeredSeconds :type "Float (double-precision)") (InputAction :type "InputAction Object Reference" :default "/Game/Jiale/Input/IA_Reload.IA_Reload"))
  ;[1 1 1] 换弹
  (:`Triggered`
    (if (`self.isReloadReady`)
      (`self.Event Reload Both`)
      (set `self.isReloadReady` false)
      (else
        (set `self.isReloadReady` true)))))

(fn `UserConstructionScript`)