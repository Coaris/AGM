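; One-shot swinging door that opens away from the player when BP_Bill overlaps its collision.
; The sign of the dot product between the player-to-door offset and the door's forward vector selects one of two timelines.
; Each timeline yaws the DoorCloser component up to 90 degrees in opposite directions.
; The used flag is set before the cast, so any first overlapping actor consumes the trigger.
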(event `self.Collision.OnComponentBeginOverlap`
  (params (OverlappedComponent :type "PrimitiveComponent Object Reference") (OtherActor :type "Actor Object Reference") (OtherComp :type "PrimitiveComponent Object Reference") (OtherBodyIndex :type Integer) (bFromSweep :type Boolean) (SweepResult :type "HitResult Structure (by ref)"))
  (if (not (`self.isUsed`))
    (set `self.isUsed` true)
    (cast `/Game/Jiale/BP/Bill/BP_Bill` OtherActor)
    (if (<= (`KismetMathLibrary.Dot_VectorVector` (- (`self.K2_GetActorLocation` (`GameplayStatics.GetPlayerPawn` 0)) (`self.K2_GetActorLocation`)) (`SceneComponent.GetForwardVector` (`self.DefaultSceneRoot`))) 0.0)
      (bind (_direction _newtrack_0) (`Timeline|OpenDOor` :!via `PlayFromStart`)
        (:`Update`
          (`SceneComponent.K2_SetRelativeRotation` (`self.DoorCloser`) (`KismetMathLibrary.MakeRotator` 0.0 0.0 (* _newtrack_0 -90.0)) false false)))
      (else
        (bind (_direction_2 _newtrack_0_2) (`Timeline|Timeline` :!via `PlayFromStart`)
          (:`Update`
            (`SceneComponent.K2_SetRelativeRotation` (`self.DoorCloser`) (`KismetMathLibrary.MakeRotator` 0.0 0.0 (* _newtrack_0_2 90.0)) false false)))))))

(fn `UserConstructionScript`)